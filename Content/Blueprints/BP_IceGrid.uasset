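; Grid actor that spawns BP_IceBlocks and drops regions cut out by the player's traveled path.
; Blocks live in nested arrays split by coordinate sign; path segments become edge flags keyed by endpoint sums.
; Flood4 runs an iteration-limited recursive flood fill from four cells around a point, keeping the smallest non-empty region.
; Regions under MaxCut fall, then the player's trail points and particles are cleared.
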(event `Flood4Event`
  (params (PointsTraveled :type "Array of Vector Structure") (X :type Integer) (Y :type Integer))
  (`self.Flood4` PointsTraveled X Y))

(event `self.ReceiveBeginPlay`
  (bind (_iceblocks_positivex _iceblocks_negativex) (break `/Game/Blueprints/S_Grid` (`self.IceBlocks`)))
  (bind (_iceblocks_positivex_2 _iceblocks_negativex_2) (break `/Game/Blueprints/S_Grid` (`self.IceBlocks`)))
  (bind _returnvalue (/ (`self.NumberInX`) 2))
  (`KismetArrayLibrary.Array_Set` _iceblocks_positivex_2 _returnvalue (struct) true)
  (`KismetArrayLibrary.Array_Set` _iceblocks_negativex_2 (+ _returnvalue 1) (struct) true)
  (bind (_current_point _total_points _0_1_phase _poly_center) (`/Engine/ArtTools/RenderToTexture/Macros/RenderToTextureMacros.2D Grid Execution Macro` 100.0 (`self.K2_GetActorLocation`) (`self.NumberInX`) (`self.NumberInY`))
    (:`Per Poly Execution`
      (bind _returnvalue_2 (`|SpawnActorFromClass` "/Game/Blueprints/BP_IceBlock.BP_IceBlock_C" (`KismetMathLibrary.MakeTransform` _poly_center) "Undefined" "OverrideRootScale" null null))
      (bind (_returnvalue_x _returnvalue_y) (`KismetMathLibrary.BreakVector` (`self.K2_GetActorLocation` _returnvalue_2)))
      (bind _returnvalue_3 (`KismetMathLibrary.Round` (/ (`KismetMathLibrary.GridSnap_Float` (- _returnvalue_x 50.0) 100.0) 100.0)))
      (bind (_output_positivey _output_negativey) (break `/Game/Blueprints/S_Y` (`|GetArrayItem` (select `bool` (< _returnvalue_3 0) :`false` _iceblocks_positivex :`true` _iceblocks_negativex) (`KismetMathLibrary.Abs_Int` _returnvalue_3))))
      (bind _returnvalue_4 (`KismetMathLibrary.Round` (/ (`KismetMathLibrary.GridSnap_Float` (- _returnvalue_y 50.0) 100.0) 100.0)))
      (`KismetArrayLibrary.Array_Set` (select `bool` (< _returnvalue_4 0) :`false` _output_positivey :`true` _output_negativey) (`KismetMathLibrary.Abs_Int` _returnvalue_4) _returnvalue_2 true))))

(fn `BlockExists`
  (params (X :type Integer) (Y :type Integer))
  (returns (Exists :type Boolean))
  (bind (_iceblocks_positivex _iceblocks_negativex) (break `/Game/Blueprints/S_Grid` (`self.IceBlocks`)))
  (bind (_output_positivey _output_negativey) (break `/Game/Blueprints/S_Y` (`|GetArrayItem` (select `bool` (< X 0) :`false` _iceblocks_positivex :`true` _iceblocks_negativex) (`KismetMathLibrary.Abs_Int` X))))
  (return (`KismetSystemLibrary.IsValid` (`|GetArrayItem` (select `bool` (< Y 0) :`false` _output_positivey :`true` _output_negativey) (`KismetMathLibrary.Abs_Int` Y)))))

(fn `Check4`
  (params (X :type Integer) (Y :type Integer))
  (returns (`4Exists` :type Boolean))
  (bind _returnvalue (- X 1))
  (bind _returnvalue_2 (- Y 1))
  (return (and (`self.BlockExists` X Y) (`self.BlockExists` X _returnvalue_2) (`self.BlockExists` _returnvalue Y) (`self.BlockExists` _returnvalue _returnvalue_2))))

(fn `CheckEmpty`
  (params (X :type Integer) (Y :type Integer))
  (returns (IsEmpty :type Boolean))
  (bind _returnvalue (- X 1))
  (bind _returnvalue_2 (- Y 1))
  (return (not (or (`self.BlockExists` X Y) (`self.BlockExists` X _returnvalue_2) (`self.BlockExists` _returnvalue Y) (`self.BlockExists` _returnvalue _returnvalue_2)))))

(fn `ConvertToEdges`
  (params (Points :type "Array of Vector Structure"))
  (returns (Edges :type "/Game/Blueprints/S_Edge Structure"))
  (locals (EdgesLocal :type "/Game/Blueprints/S_Edge Structure"))
  (bind (_edgeslocal_positive _edgeslocal_negative) (break `/Game/Blueprints/S_Edge` (`local.EdgesLocal`)))
  (for (_array_element _array_index) Points
    (bind _returnvalue (+ _array_index 1))
    (if (< _returnvalue (`KismetArrayLibrary.Array_Length` Points))
      (bind (_returnvalue_x _returnvalue_y) (`KismetMathLibrary.BreakVector` (+ _array_element (`|GetArrayItem` Points _returnvalue))))
      (bind _returnvalue_2 (`KismetMathLibrary.Round` _returnvalue_x))
      (bind _returnvalue_3 (select `bool` (< _returnvalue_2 0) :`false` _edgeslocal_positive :`true` _edgeslocal_negative))
      (bind _returnvalue_4 (`KismetMathLibrary.Abs_Int` _returnvalue_2))
      (if (not (> (`KismetArrayLibrary.Array_Length` _returnvalue_3) _returnvalue_4))
        (`KismetArrayLibrary.Array_Set` _returnvalue_3 _returnvalue_4 (struct) true))
      (bind (_output_positive _output_negative) (break `/Game/Blueprints/S_Edge2` (`|GetArrayItem` _returnvalue_3 _returnvalue_4)))
      (bind _returnvalue_5 (`KismetMathLibrary.Round` _returnvalue_y))
      (`KismetArrayLibrary.Array_Set` (select `bool` (< _returnvalue_5 0) :`false` _output_positive :`true` _output_negative) (`KismetMathLibrary.Abs_Int` _returnvalue_5) true true)))
  (return (`local.EdgesLocal`)))

(fn `EdgeExists`
  (params (X1 :type Integer) (Y1 :type Integer) (X2 :type Integer) (Y2 :type Integer) (Edges :type "/Game/Blueprints/S_Edge Structure"))
  (returns (Exists :type Boolean))
  (bind _returnvalue (+ X1 X2))
  (bind _returnvalue_2 (+ Y1 Y2))
  (bind _returnvalue_3 (`KismetMathLibrary.Abs_Int` _returnvalue))
  (bind _returnvalue_4 (`KismetMathLibrary.Abs_Int` _returnvalue_2))
  (bind _returnvalue_5 (select `bool` (< _returnvalue 0) :`false` Edges_Positive_3_58F62108174756CB22668581348218FA :`true` Edges_Negative_5_E135ACDD0644DB4599BAA58F54829F77))
  (bind (_output_positive _output_negative) (break `/Game/Blueprints/S_Edge2` (`|GetArrayItem` _returnvalue_5 _returnvalue_3)))
  (bind _returnvalue_6 (select `bool` (< _returnvalue_2 0) :`false` _output_positive :`true` _output_negative))
  (if (> (`KismetArrayLibrary.Array_Length` _returnvalue_5) _returnvalue_3)
    (if (> (`KismetArrayLibrary.Array_Length` _returnvalue_6) _returnvalue_4)
      (return (`|GetArrayItem` _returnvalue_6 _returnvalue_4))
      (else
        _)))
  (return false))

(fn `Flood4`
  (params (PointsTraveled :type "Array of Vector Structure") (X :type Integer) (Y :type Integer))
  (locals (Points :type "Array of Vector Structure") (xLocal :type Integer) (yLocal :type Integer) (Blocks :type "Array of /Game/Blueprints/BP_IceBlock Object Reference") (Edges :type "/Game/Blueprints/S_Edge Structure"))
  (bind _returnvalue (`KismetArrayLibrary.Array_Length` (`self.FilledBlocks`)))
  (bind _returnvalue_2 (`KismetArrayLibrary.Array_Length` (`self.FilledBlocks`)))
  (bind _returnvalue_3 (`KismetArrayLibrary.Array_Length` (`self.FilledBlocks`)))
  (bind _returnvalue_4 (`KismetArrayLibrary.Array_Length` (`self.FilledBlocks`)))
  (bind _returnvalue_5 (`KismetArrayLibrary.Array_Length` (`local.Blocks`)))
  (bind _edges (`self.ConvertToEdges` PointsTraveled))
  (set `local.Edges` _edges)
  (set `local.xLocal` X)
  (set `local.yLocal` Y)
  (`|ExecutionSequence`
    (:`then_0`
      (`KismetArrayLibrary.Array_Clear` (`self.FilledBlocks`))
      (`self.FloodFill` (`local.Edges`) (`local.xLocal`) (`local.yLocal`) (`self.Iterations`))
      (if (> (`KismetArrayLibrary.Array_Length` (`local.Blocks`)) 0)
        (if (and (> _returnvalue_2 0) (< _returnvalue_2 (`KismetArrayLibrary.Array_Length` (`local.Blocks`))))
          (set `local.Blocks` (`self.FilledBlocks`) :!label _label))
        (else
          (goto _label))))
    (:`then_1`
      (`KismetArrayLibrary.Array_Clear` (`self.FilledBlocks`))
      (`self.FloodFill` (`local.Edges`) (`local.xLocal`) (- (`local.yLocal`) 1) (`self.Iterations`))
      (if (> (`KismetArrayLibrary.Array_Length` (`local.Blocks`)) 0)
        (if (and (> _returnvalue_3 0) (< _returnvalue_3 (`KismetArrayLibrary.Array_Length` (`local.Blocks`))))
          (set `local.Blocks` (`self.FilledBlocks`) :!label _label_2))
        (else
          (goto _label_2))))
    (:`then_2`
      (`KismetArrayLibrary.Array_Clear` (`self.FilledBlocks`))
      (`self.FloodFill` (`local.Edges`) (- (`local.xLocal`) 1) (`local.yLocal`) (`self.Iterations`))
      (if (> (`KismetArrayLibrary.Array_Length` (`local.Blocks`)) 0)
        (if (and (> _returnvalue_4 0) (< _returnvalue_4 (`KismetArrayLibrary.Array_Length` (`local.Blocks`))))
          (set `local.Blocks` (`self.FilledBlocks`) :!label _label_3))
        (else
          (goto _label_3))))
    (:`then_3`
      (`KismetArrayLibrary.Array_Clear` (`self.FilledBlocks`))
      (`self.FloodFill` (`local.Edges`) (- (`local.xLocal`) 1) (- (`local.yLocal`) 1) (`self.Iterations`))
      (if (> (`KismetArrayLibrary.Array_Length` (`local.Blocks`)) 0)
        (if (and (> _returnvalue 0) (< _returnvalue (`KismetArrayLibrary.Array_Length` (`local.Blocks`))))
          (set `local.Blocks` (`self.FilledBlocks`) :!label _label_4))
        (else
          (goto _label_4))))
    (:`then_4`
      (if (and (< _returnvalue_5 (`self.MaxCut`)) (> _returnvalue_5 0))
        (for _array_element (`local.Blocks`)
          (`/Game/Blueprints/BP_IceBlock.Fall` _array_element))
        (bind _asbp_player_pawn (cast `/Game/Blueprints/BP_PlayerPawn` (`GameplayStatics.GetPlayerPawn` 0)))
        (`KismetArrayLibrary.Array_Clear` (`/Game/Blueprints/BP_PlayerPawn.TraveledPoints` _asbp_player_pawn))
        (bind _particlesystem (`/Game/Blueprints/BP_PlayerPawn.ParticleSystem` _asbp_player_pawn))
        (for _array_element_2 _particlesystem
          (`ActorComponent.K2_DestroyComponent` _array_element_2))
        (`KismetArrayLibrary.Array_Clear` _particlesystem)))))

(fn `FloodFill`
  (params (Edges :type "/Game/Blueprints/S_Edge Structure") (X :type Integer) (Y :type Integer) (Iterations :type Integer))
  (locals (xLocal :type Integer) (yLocal :type Integer) (IterationLocal :type Integer) (PointsLocal :type "Array of Vector Structure") (EdgesLocal :type "/Game/Blueprints/S_Edge Structure"))
  (bind (_iceblocks_positivex _iceblocks_negativex) (break `/Game/Blueprints/S_Grid` (`self.IceBlocks`)))
  (bind _xlocal (`local.xLocal`))
  (bind _ylocal (`local.yLocal`))
  (bind _xlocal_2 (`local.xLocal`))
  (bind _ylocal_2 (`local.yLocal`))
  (bind _xlocal_3 (`local.xLocal`))
  (bind _ylocal_3 (`local.yLocal`))
  (bind _xlocal_4 (`local.xLocal`))
  (bind _ylocal_4 (`local.yLocal`))
  (bind _returnvalue (+ (`local.yLocal`) 1))
  (bind _returnvalue_2 (+ (`local.xLocal`) 1))
  (bind (_output_positivey _output_negativey) (break `/Game/Blueprints/S_Y` (`|GetArrayItem` (select `bool` (< _xlocal 0) :`false` _iceblocks_positivex :`true` _iceblocks_negativex) (`KismetMathLibrary.Abs_Int` _xlocal))))
  (set `local.xLocal` X)
  (set `local.yLocal` Y)
  (set `local.IterationLocal` Iterations)
  (set `local.EdgesLocal` Edges)
  (if (and (> Iterations 0) (`self.BlockExists` (`local.xLocal`) (`local.yLocal`)))
    (bind _returnvalue_3 (`KismetArrayLibrary.Array_AddUnique` (`self.FilledBlocks`) (`|GetArrayItem` (select `bool` (< _ylocal 0) :`false` _output_positivey :`true` _output_negativey) (`KismetMathLibrary.Abs_Int` _ylocal))))
    (if (== _returnvalue_3 -1)
      (return)
      (else
        (`|ExecutionSequence`
          (:`then_0`
            (bind _exists (`self.EdgeExists` _returnvalue_2 _ylocal_3 _returnvalue_2 (+ _ylocal_3 1) (`local.EdgesLocal`)))
            (if (not _exists)
              (`self.FloodFill` (`local.EdgesLocal`) (+ (`local.xLocal`) 1) (`local.yLocal`) (- (`local.IterationLocal`) 1))))
          (:`then_1`
            (bind _exists_2 (`self.EdgeExists` _xlocal_2 _ylocal_2 _xlocal_2 (+ _ylocal_2 1) (`local.EdgesLocal`)))
            (if (not _exists_2)
              (`self.FloodFill` (`local.EdgesLocal`) (+ (`local.xLocal`) -1) (`local.yLocal`) (- (`local.IterationLocal`) 1))))
          (:`then_2`
            (bind _exists_3 (`self.EdgeExists` _xlocal_4 _ylocal_4 (+ _xlocal_4 1) _ylocal_4 (`local.EdgesLocal`)))
            (if (not _exists_3)
              (`self.FloodFill` (`local.EdgesLocal`) (`local.xLocal`) (+ (`local.yLocal`) -1) (- (`local.IterationLocal`) 1))))
          (:`then_3`
            (bind _exists_4 (`self.EdgeExists` _xlocal_3 _returnvalue (+ _xlocal_3 1) _returnvalue (`local.EdgesLocal`)))
            (if (not _exists_4)
              (`self.FloodFill` (`local.EdgesLocal`) (`local.xLocal`) (+ (`local.yLocal`) 1) (- (`local.IterationLocal`) 1)))))))
    (else
      (return))))

(fn `UserConstructionScript`)