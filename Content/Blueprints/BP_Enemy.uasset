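; BP_Enemy is a hopping cube enemy that chases the player and reloads StartMap when it hits the player pawn.
; Tick turns the actor's yaw to face the player, while a looping timer calls Jump.
; Jump applies a mass-independent forward-and-up impulse to the Cube.
; When destroyed, it adds its Points to the score through MyPlayerController.
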(event `self.ReceiveHit`
  (params (MyComp :type "PrimitiveComponent Object Reference") (Other :type "Actor Object Reference") (OtherComp :type "PrimitiveComponent Object Reference") (bSelfMoved :type Boolean) (HitLocation :type "Vector Structure") (HitNormal :type "Vector Structure") (NormalImpulse :type "Vector Structure") (Hit :type "HitResult Structure (by ref)"))
  (cast `/Game/Blueprints/BP_PlayerPawn` Other)
  (`GameplayStatics.OpenLevel` "StartMap"))

(event `self.ReceiveBeginPlay`
  (`KismetSystemLibrary.K2_SetTimer` null "Jump" 1.5 true))

(event `self.ReceiveTick`
  (params (DeltaSeconds :type "Float (single-precision)"))
  (bind (_returnvalue_roll _returnvalue_pitch _returnvalue_yaw) (`KismetMathLibrary.BreakRotator` (`KismetMathLibrary.FindLookAtRotation` (`self.K2_GetActorLocation`) (`self.K2_GetActorLocation` (`GameplayStatics.GetPlayerPawn` 0)))))
  (`self.K2_SetActorRotation` (`KismetMathLibrary.MakeRotator` 0.0 0.0 _returnvalue_yaw)))

(event `self.ReceiveDestroyed`
  (`/Game/Blueprints/MyPlayerController.IncreaseScore` (cast `/Game/Blueprints/MyPlayerController` (`GameplayStatics.GetPlayerController` 0) :!pure true) (`self.Points`)))

(fn `Jump`
  (bind _cube (`self.Cube`))
  (`PrimitiveComponent.AddImpulse` _cube (* (+ (`SceneComponent.GetForwardVector` _cube) (0.0 0.0 2.0)) 300.0) "None" true))

(fn `UserConstructionScript`)