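; BP_Enemy2 is a shooting enemy that destroys the player pawn on contact and awards its Points when destroyed.
; Each tick it sets its yaw to face the player pawn.
; A looping timer started at BeginPlay calls Shoot, which spawns a BP_Bullet just ahead of it along its forward vector.
; On destruction it passes Points to IncreaseScore on MyPlayerController.
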(event `self.ReceiveHit`
  (params (MyComp :type "PrimitiveComponent Object Reference") (Other :type "Actor Object Reference") (OtherComp :type "PrimitiveComponent Object Reference") (bSelfMoved :type Boolean) (HitLocation :type "Vector Structure") (HitNormal :type "Vector Structure") (NormalImpulse :type "Vector Structure") (Hit :type "HitResult Structure (by ref)"))
  (bind _asbp_player_pawn (cast `/Game/Blueprints/BP_PlayerPawn` Other))
  (`self.K2_DestroyActor` _asbp_player_pawn))

(event `self.ReceiveBeginPlay`
  (`KismetSystemLibrary.K2_SetTimer` null "Shoot" 2.0 true))

(event `self.ReceiveTick`
  (params (DeltaSeconds :type "Float (single-precision)"))
  (bind (_returnvalue_roll _returnvalue_pitch _returnvalue_yaw) (`KismetMathLibrary.BreakRotator` (`KismetMathLibrary.FindLookAtRotation` (`self.K2_GetActorLocation`) (`self.K2_GetActorLocation` (`GameplayStatics.GetPlayerPawn` 0)))))
  (`self.K2_SetActorRotation` (`KismetMathLibrary.MakeRotator` 0.0 0.0 _returnvalue_yaw)))

(event `self.ReceiveDestroyed`
  (`/Game/Blueprints/MyPlayerController.IncreaseScore` (cast `/Game/Blueprints/MyPlayerController` (`GameplayStatics.GetPlayerController` 0) :!pure true) (`self.Points`)))

(fn `Shoot`
  (bind (_returnvalue_location _returnvalue_rotation) (`KismetMathLibrary.BreakTransform` (`self.GetTransform`)))
  (`|SpawnActorFromClass` "/Game/Blueprints/BP_Bullet.BP_Bullet_C" (`KismetMathLibrary.MakeTransform` (+ _returnvalue_location (* (`self.GetActorForwardVector`) 100.0)) _returnvalue_rotation) "Undefined" "OverrideRootScale" null null))

(fn `UserConstructionScript`)