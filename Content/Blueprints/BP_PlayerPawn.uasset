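; Player pawn that moves continuously across a grid in 100-unit steps, with A and D queuing a timeline-animated 90-degree turn between steps.
; Each step records the grid-snapped cell in TraveledPoints and checks whether it was visited before.
; On a revisit, it extracts the closed loop, passes it to BP_IceGrid's FloodFill, enables physics on the returned meshes and restarts the trail.
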(event `Key|A`
  (params (Key :type "Key Structure"))
  (:`Pressed`
    (set `self.RotateRight` false)
    (set `self.RotateLeft` true)))

(event `Key|D`
  (params (Key :type "Key Structure"))
  (:`Pressed`
    (set `self.RotateRight` true)
    (set `self.RotateLeft` false)))

(event `self.ReceiveBeginPlay`
  (bind (_returnvalue_x _returnvalue_y) (`KismetMathLibrary.BreakVector` (`self.K2_GetActorLocation`)))
  (bind (_returnvalue_x_2 _returnvalue_y_2) (`KismetMathLibrary.BreakVector` (`self.K2_GetActorLocation`)))
  (bind (_returnvalue_x_3 _returnvalue_y_3) (`KismetMathLibrary.BreakVector` (`self.K2_GetActorLocation`)))
  (bind (_returnvalue_location _returnvalue_rotation) (`KismetMathLibrary.BreakTransform` (`self.GetTransform`)))
  (bind (_returnvalue_roll _returnvalue_pitch _returnvalue_yaw) (`KismetMathLibrary.BreakRotator` (`self.K2_GetActorRotation`)))
  (bind (_returnvalue_roll_2 _returnvalue_pitch_2) (`KismetMathLibrary.BreakRotator` (`self.K2_GetActorRotation`)))
  (bind (_returnvalue_x_4 _returnvalue_y_4) (`KismetMathLibrary.BreakVector` (`self.K2_GetActorLocation`)))
  (`KismetSystemLibrary.MoveComponentTo` (`self.Cube`) (+ (* (`SceneComponent.GetForwardVector` (`self.Cube`)) 100) _returnvalue_location) _returnvalue_rotation false false (`self.MoveTime`) :!label _label)
  (for (_array_element _array_index) (`self.TraveledPoints`)
    (if (== _array_element (`KismetMathLibrary.MakeVector` (/ (`KismetMathLibrary.GridSnap_Float` _returnvalue_x_4 100.0) 100.0) (/ (`KismetMathLibrary.GridSnap_Float` _returnvalue_y_4 100.0) 100.0)))
      (set `self.Index` _array_index)
      (break)))
  (if (== (`self.Index`) -1)
    (`KismetArrayLibrary.Array_Add` (`self.TraveledPoints`) (`KismetMathLibrary.MakeVector` (/ (`KismetMathLibrary.GridSnap_Float` _returnvalue_x 100.0) 100.0) (/ (`KismetMathLibrary.GridSnap_Float` _returnvalue_y 100.0) 100.0)))
    (else
      (`KismetArrayLibrary.Array_Add` (`self.TraveledPoints`) (`KismetMathLibrary.MakeVector` (/ (`KismetMathLibrary.GridSnap_Float` _returnvalue_x_2 100.0) 100.0) (/ (`KismetMathLibrary.GridSnap_Float` _returnvalue_y_2 100.0) 100.0)))
      (for (_array_element_2 _array_index_2) (`self.TraveledPoints`)
        (if (>= _array_index_2 (`self.Index`))
          (`KismetArrayLibrary.Array_Add` (`self.Loop`) _array_element_2)))
      (`KismetArrayLibrary.Array_Clear` (`self.TraveledPoints`))
      (bind _outactors (`GameplayStatics.GetAllActorsOfClass` "/Game/Blueprints/BP_IceGrid.BP_IceGrid_C"))
      (bind _blocks (`/Game/Blueprints/BP_IceGrid.FloodFill` (`|GetArrayItem` _outactors) (`self.Loop`) (`KismetMathLibrary.Round` (/ (`KismetMathLibrary.GridSnap_Float` _returnvalue_x_3 100.0) 100.0)) (`KismetMathLibrary.Round` (/ (`KismetMathLibrary.GridSnap_Float` _returnvalue_y_3 100.0) 100.0)) 5))
      (`KismetArrayLibrary.Array_Clear` (`self.Loop`))
      (for _array_element_3 _blocks
        (`PrimitiveComponent.SetSimulatePhysics` (`StaticMeshActor.StaticMeshComponent` _array_element_3) true))
      (set `self.Index` -1)))
  (if (or (`self.RotateRight`) (`self.RotateLeft`))
    (set `self.Yaw` _returnvalue_yaw)
    (set `self.DeltaYaw` (`KismetMathLibrary.SelectFloat` 90.0 -90.0 (`self.RotateRight`)))
    (set `self.RotateRight` false)
    (set `self.RotateLeft` false)
    (bind (_direction _fraction) (`Timeline|Rotation` :!via `PlayFromStart`)
      (:`Update`
        (`self.K2_SetActorRotation` (`KismetMathLibrary.MakeRotator` _returnvalue_roll_2 _returnvalue_pitch_2 (+ (* _fraction (`self.DeltaYaw`)) (`self.Yaw`)))))
      (:`Finished`
        (goto _label)))
    (else
      (goto _label))))

(fn `UserConstructionScript`)