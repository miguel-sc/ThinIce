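; Boss enemy that hops toward the player and bursts into smaller enemies when destroyed.
; It yaws to face the player every tick, and a looping timer launches its cube forward and upward with velocity-change impulses.
; Hitting the player pawn reloads StartMap.
; On destruction it awards points and spawns eight BP_Enemy actors in a surrounding ring, each flung outward and upward.
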(event `self.ReceiveHit`
  (params (MyComp :type "PrimitiveComponent Object Reference") (Other :type "Actor Object Reference") (OtherComp :type "PrimitiveComponent Object Reference") (bSelfMoved :type Boolean) (HitLocation :type "Vector Structure") (HitNormal :type "Vector Structure") (NormalImpulse :type "Vector Structure") (Hit :type "HitResult Structure (by ref)"))
  (cast `/Game/Blueprints/BP_PlayerPawn` Other)
  (`GameplayStatics.OpenLevel` "StartMap"))

(event `self.ReceiveBeginPlay`
  (`KismetSystemLibrary.K2_SetTimer` null "Jump" 1.5 true))

(event `self.ReceiveTick`
  (params (DeltaSeconds :type "Float (single-precision)"))
  (bind (_returnvalue_roll _returnvalue_pitch _returnvalue_yaw) (`KismetMathLibrary.BreakRotator` (`KismetMathLibrary.FindLookAtRotation` (`self.K2_GetActorLocation`) (`self.K2_GetActorLocation` (`GameplayStatics.GetPlayerPawn` 0)))))
  (`self.K2_SetActorRotation` (`KismetMathLibrary.MakeRotator` 0.0 0.0 _returnvalue_yaw)))

(event `self.ReceiveDestroyed`
  (`/Game/Blueprints/MyPlayerController.IncreaseScore` (cast `/Game/Blueprints/MyPlayerController` (`GameplayStatics.GetPlayerController` 0) :!pure true) (`self.Points`))
  (`|ExecutionSequence`
    (:`then_0`
      (bind _returnvalue (`|SpawnActorFromClass` "/Game/Blueprints/BP_Enemy.BP_Enemy_C" (`KismetMathLibrary.MakeTransform` (+ (`self.K2_GetActorLocation`) (100.0 0.0 0.0))) "AlwaysSpawn" "OverrideRootScale" null null))
      (`PrimitiveComponent.AddImpulse` (`/Game/Blueprints/BP_Enemy.Cube` _returnvalue) (300.0 0.0 800.0) "None" true))
    (:`then_1`
      (bind _returnvalue_2 (`|SpawnActorFromClass` "/Game/Blueprints/BP_Enemy.BP_Enemy_C" (`KismetMathLibrary.MakeTransform` (+ (`self.K2_GetActorLocation`) (100.0 100.0 0.0))) "AlwaysSpawn" "OverrideRootScale" null null))
      (`PrimitiveComponent.AddImpulse` (`/Game/Blueprints/BP_Enemy.Cube` _returnvalue_2) (300.0 300.0 800.0) "None" true))
    (:`then_2`
      (bind _returnvalue_3 (`|SpawnActorFromClass` "/Game/Blueprints/BP_Enemy.BP_Enemy_C" (`KismetMathLibrary.MakeTransform` (+ (`self.K2_GetActorLocation`) (100.0 -100.0 0.0))) "AlwaysSpawn" "OverrideRootScale" null null))
      (`PrimitiveComponent.AddImpulse` (`/Game/Blueprints/BP_Enemy.Cube` _returnvalue_3) (300.0 -300.0 800.0) "None" true))
    (:`then_3`
      (bind _returnvalue_4 (`|SpawnActorFromClass` "/Game/Blueprints/BP_Enemy.BP_Enemy_C" (`KismetMathLibrary.MakeTransform` (+ (`self.K2_GetActorLocation`) (-100.0 0.0 0.0))) "AlwaysSpawn" "OverrideRootScale" null null))
      (`PrimitiveComponent.AddImpulse` (`/Game/Blueprints/BP_Enemy.Cube` _returnvalue_4) (-300.0 0.0 800.0) "None" true))
    (:`then_4`
      (bind _returnvalue_5 (`|SpawnActorFromClass` "/Game/Blueprints/BP_Enemy.BP_Enemy_C" (`KismetMathLibrary.MakeTransform` (+ (`self.K2_GetActorLocation`) (-100.0 100.0 0.0))) "AlwaysSpawn" "OverrideRootScale" null null))
      (`PrimitiveComponent.AddImpulse` (`/Game/Blueprints/BP_Enemy.Cube` _returnvalue_5) (-300.0 300.0 800.0) "None" true))
    (:`then_5`
      (bind _returnvalue_6 (`|SpawnActorFromClass` "/Game/Blueprints/BP_Enemy.BP_Enemy_C" (`KismetMathLibrary.MakeTransform` (+ (`self.K2_GetActorLocation`) (-100.0 -100.0 0.0))) "AlwaysSpawn" "OverrideRootScale" null null))
      (`PrimitiveComponent.AddImpulse` (`/Game/Blueprints/BP_Enemy.Cube` _returnvalue_6) (-300.0 -300.0 800.0) "None" true))
    (:`then_6`
      (bind _returnvalue_7 (`|SpawnActorFromClass` "/Game/Blueprints/BP_Enemy.BP_Enemy_C" (`KismetMathLibrary.MakeTransform` (+ (`self.K2_GetActorLocation`) (0.0 100.0 0.0))) "AlwaysSpawn" "OverrideRootScale" null null))
      (`PrimitiveComponent.AddImpulse` (`/Game/Blueprints/BP_Enemy.Cube` _returnvalue_7) (0.0 300.0 800.0) "None" true))
    (:`then_7`
      (bind _returnvalue_8 (`|SpawnActorFromClass` "/Game/Blueprints/BP_Enemy.BP_Enemy_C" (`KismetMathLibrary.MakeTransform` (+ (`self.K2_GetActorLocation`) (0.0 -100.0 0.0))) "AlwaysSpawn" "OverrideRootScale" null null))
      (`PrimitiveComponent.AddImpulse` (`/Game/Blueprints/BP_Enemy.Cube` _returnvalue_8) (0.0 -300.0 800.0) "None" true))))

(fn `Jump`
  (bind _cube (`self.Cube`))
  (`PrimitiveComponent.AddImpulse` _cube (* (+ (`SceneComponent.GetForwardVector` _cube) (0.0 0.0 2.0)) 300.0) "None" true))

(fn `UserConstructionScript`)