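; Player controller that manages score, UI widgets and level switching between StartMap and MainMap.
; BeginPlay creates the score HUD; helper functions show the start menu and temporary instructions on request.
; IncreaseScore increments Score by one, ignoring its Points input, and shows victory on the HUD at MaxScore.
; StartGame input opens MainMap; EndGame returns to StartMap from MainMap, otherwise quits.
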(event `self.ReceiveBeginPlay`
  (bind _returnvalue (`|CreateWidget` "/Game/UI/ScoreHUD.ScoreHUD_C" self))
  (set `self.HUDRef` _returnvalue)
  (`UserWidget.AddToViewport` _returnvalue 0))

(event `InputAction|EndGame`
  (params (Key :type "Key Structure"))
  (:`Pressed`
    (bind _returnvalue (`GameplayStatics.GetCurrentLevelName` true))
    (if (`KismetStringLibrary.EqualEqual_StrStr` _returnvalue "MainMap")
      (`GameplayStatics.OpenLevel` "StartMap")
      (`Widget.SetVisibility` (`/Game/UI/ScoreHUD.VictoryText` (`self.HUDRef`)) "Hidden")
      (else
        (`KismetSystemLibrary.QuitGame` null "Quit")))))

(event `InputAction|StartGame`
  (params (Key :type "Key Structure"))
  (:`Pressed`
    (`GameplayStatics.OpenLevel` "MainMap")))

(fn `IncreaseScore`
  (params (Points :type Integer))
  (bind _result (`/Engine/EditorBlueprintResources/StandardMacros.IncrementInt` (`self.Score`))
    (:`  `
      (if (>= _result (`self.MaxScore`))
        (`/Game/UI/ScoreHUD.ShowVictory` (`self.HUDRef`)))
      (return))))

(fn `ShowInstructions`
  (`/Game/UI/ScoreHUD.TemporaryInstructions` (`self.HUDRef`)))

(fn `ShowStartMenuUI`
  (bind _returnvalue (`|CreateWidget` "/Game/UI/StartMapUI.StartMapUI_C"))
  (`UserWidget.AddToViewport` _returnvalue 0)
  (return))

(fn `UserConstructionScript`)